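; Player character for a three-lane endless runner that constantly runs along control yaw, with Enhanced Input jump, slide and lane changes.
; Slide applies a downward impulse; when grounded and moving, it plays a montage while briefly disabling input and ignoring Destructible collision.
; Lane input sets a clamped target index, but the timeline lerps Y toward the current index's position, adopting the target only on finish.
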(event Custom|Change%20Lanes
  (params (Shift%20Lanes :type Integer))
  (bind _returnvalue (Transformation|GetActorLocation))
  (bind (_x _y _z) (Math|Vector|BreakVector _returnvalue))
  ;[1 1 1] Change Lanes
  (Variables|Default|SetTarget%20Lane%20Index (Math|Integer|Clamp(Integer) (+ Shift%20Lanes (Variables|Default|GetCurrent%20Lane%20Index)) 0 2))
  (Variables|Default|SetCurrent%20Y (.Y (Math|Vector|BreakVector (Transformation|GetActorLocation))))
  (bind _change_lane (Timeline|Transition PlayFromStart)
    (:Update
      (Transformation|SetActorLocation (Math|Vector|MakeVector _x (Math|Float|Lerp (Variables|Default|GetCurrent%20Y) (Utilities|Array|Get(acopy) (Variables|Default|GetLane%20Position) (Variables|Default|GetCurrent%20Lane%20Index)) _change_lane) _z) false false))
    (:Finished
      (Variables|Default|SetCurrent%20Lane%20Index (Variables|Default|GetTarget%20Lane%20Index)))))

(event Input|EnhancedActionEvents|EnhancedInputActionJump_IA
  (params (ActionValue :type Boolean) (ElapsedSeconds :type Float%20%28double-precision%29) (TriggeredSeconds :type Float%20%28double-precision%29) (InputAction :type Input%20Action%20Object%20Reference :default "/Game/Runner/Blueprints/Input/Jump_IA.Jump_IA"))
  (:Started
    (Character|Jump)))

(event Input|EnhancedActionEvents|EnhancedInputActionSlide_IA
  (params (ActionValue :type Boolean) (ElapsedSeconds :type Float%20%28double-precision%29) (TriggeredSeconds :type Float%20%28double-precision%29) (InputAction :type Input%20Action%20Object%20Reference :default "/Game/Runner/Blueprints/Input/Slide_IA.Slide_IA"))
  (bind _charactermovement (Variables|Character|GetCharacterMovement))
  ;[1 1 1] Sliding
  (Physics|AddImpulse (Variables|Character|GetCharacterMovement) "0.000000,0.000000,-1000.000000" true)
  (if (and (> (Math|Vector|VectorLength (Variables|/Script/Engine.MovementComponent|GetVelocity _charactermovement)) 6e+01) (not (AI|Components|NavMovement|IsFalling _charactermovement)))
    (Utilities|FlowControl|DoOnce false :!label _label
      (:Completed
        (Input|DisableInput 0)
        (Collision|SetCollisionResponsetoChannel (Variables|Collision|GetCapsuleComponent) "ECC_Destructible" "ECR_Ignore")
        (Variables|Default|SetIsSliding true)
        (Animation|Montage|MontagePlay (Components|SkeletalMesh|GetAnimInstance (Variables|Character|GetMesh)) "/Game/Runner/Animations/Running_Slide_Anim_mixamo_com_Montage.Running_Slide_Anim_mixamo_com_Montage" 1.5 "MontageLength" 0.0 true)
        (Utilities|FlowControl|Delay 0.7)
        (Input|EnableInput 0)
        (Collision|SetCollisionResponsetoChannel (Variables|Collision|GetCapsuleComponent) "ECC_Destructible" "ECR_Block")
        (Variables|Default|SetIsSliding false)
        (goto _label Reset)))))

(event Input|EnhancedActionEvents|EnhancedInputActionMove_IA
  (params (ActionValue :type Float%20%28double-precision%29) (ElapsedSeconds :type Float%20%28double-precision%29) (TriggeredSeconds :type Float%20%28double-precision%29) (InputAction :type Input%20Action%20Object%20Reference :default "/Game/Runner/Blueprints/Input/Move_IA.Move_IA"))
  ;[1 1 1] Change Lanes
  (CallFunction|ChangeLanes (Math|Float|Truncate ActionValue)))

(event EventBeginPlay
  ;[1 1 1] AddInputMapping
  (bind _asplayer_controller (Utilities|Casting|CastToPlayerController (Pawn|GetController)))
  (Utilities|IsValid (PlayerController|LocalPlayerSubsystems|GetEnhancedInputLocalPlayerSubsystem _asplayer_controller)
    (:Is%20Valid
      (Input|AddMappingContext (PlayerController|LocalPlayerSubsystems|GetEnhancedInputLocalPlayerSubsystem _asplayer_controller) "/Game/Runner/Blueprints/Input/Input_Mapping_Runner.Input_Mapping_Runner" 0 "(bIgnoreAllPressedKeysUntilRelease=True,bForceImmediately=False,bNotifyUserSettings=False)"))))

(event EventTick
  (params (DeltaSeconds :type Float%20%28single-precision%29))
  ;[1 1 1] Infinite Run
  (Pawn|Input|AddMovementInput (Math|Vector|GetForwardVector (Math|Rotator|MakeRotator 0.0 0.0 (.yaw (Pawn|GetControlRotation :!class /Script/Engine.Pawn)))) 1.0 false))

(fn ConstructionScript)