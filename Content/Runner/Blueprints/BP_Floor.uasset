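; BP_Floor is a floor segment for a runner game that triggers extension of the track as the player advances.
; When BP_Runner_Character overlaps its Box, it calls ExtendFloor on Game_Mode_Runner.
; GetAttachPoint returns the Arrow's world transform as an attach point.
; A separate AddFloor function spawns another BP_Floor at FloorAttachPoint, but the overlap event does not call it directly.
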(event OnComponentBeginOverlap(Box)
  (params (OverlappedComponent :type Primitive%20Component%20Object%20Reference) (OtherActor :type Actor%20Object%20Reference) (OtherComp :type Primitive%20Component%20Object%20Reference) (OtherBodyIndex :type Integer) (bFromSweep :type Boolean) (SweepResult :type Hit%20Result%20Structure%20%28by%20ref%29))
  (Utilities|Casting|CastToBP_Runner_Character OtherActor)
  (bind _asgame_mode_runner (Utilities|Casting|CastToGame_Mode_Runner (Game|GetGameMode)))
  (Default|ExtendFloor _asgame_mode_runner))

(event EventBeginPlay)

(event Collision|EventActorBeginOverlap
  (params (OtherActor :type Actor%20Object%20Reference)))

(event EventTick
  (params (DeltaSeconds :type Float%20%28single-precision%29)))

(fn ConstructionScript)

(fn GetAttachPoint
  (return (Transformation|GetWorldTransform (Variables|Default|GetArrow))))

(fn AddFloor
  (Game|SpawnActorfromClass "BP_Floor_C" (Variables|Default|GetFloor%20Attach%20Point) "Undefined" "MultiplyWithRoot" 0 0))